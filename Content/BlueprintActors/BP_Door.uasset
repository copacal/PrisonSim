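; BP_Door is an interactable hinged door that swings between closed and open rotations.
; Interact prints a debug message, then checks IsOpen to play Timeline_DoorOpen from the start or reverse it from the end.
; The timeline's Alpha lerps the Hinge's relative rotation between ClosedRotation and OpenRotation.
; IsOpen flips on every timeline update rather than once per interaction.
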(event EventBeginPlay)

(event Collision|EventActorBeginOverlap
  (params (OtherActor :type Actor%20Object%20Reference)))

(event EventTick
  (params (DeltaSeconds :type Float%20%28single-precision%29)))

(event EventInteract
  (Development|PrintString "Door Interacted!")
  (if (Variables|Default|GetIsOpen)
    (bind _alpha (Timeline|Timeline_DoorOpen ReverseFromEnd)
      (:Update
        (Transformation|SetRelativeRotation (Variables|Default|GetHinge) (Math|Rotator|Lerp(Rotator) (Variables|Default|GetClosedRotation) (Variables|Default|GetOpenRotation) _alpha) false false)
        (Variables|Default|SetIsOpen (not (Variables|Default|GetIsOpen)))))
    (else
      (Timeline|Timeline_DoorOpen PlayFromStart))))

(fn ConstructionScript)